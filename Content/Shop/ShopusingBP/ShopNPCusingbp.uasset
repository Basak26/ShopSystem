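; Shop NPC actor that opens the shop UI when the local player walks into its trigger box.
; On overlap it blends the player's view to itself, then waits slightly longer than the blend before creating WG_Shop with a reference to the NPC.
; The widget takes UI-only input with flushed keys and a visible cursor.
; Leaving the box only prints a message, with no view or input restore here.
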(event OnComponentBeginOverlap(ShopTriggerBox)
  (params (OverlappedComponent :type Primitive%20Component%20Object%20Reference) (OtherActor :type Actor%20Object%20Reference) (OtherComp :type Primitive%20Component%20Object%20Reference) (OtherBodyIndex :type Integer) (bFromSweep :type Boolean) (SweepResult :type Hit%20Result%20Structure%20%28by%20ref%29))
  (bind _returnvalue (Game|GetPlayerController 0))
  ;[1 1 1] Get Controller을 Cast To PlayerController로 변환하여 Target 연결
  (if (== OtherActor (Game|GetPlayerCharacter 0))
    (Development|PrintString "Hello")
    ;[1 1 1 1 12] Target: Overlap된 본인의 화면만 시점 변환
    ; Blend Time: 카메라 전환 속도
    (Game|Player|SetViewTargetwithBlend (Game|GetPlayerController 0) self 1.0 "VTBlend_Linear" 0.0 false)
    ;[1 1 1 1 12] 자연스러운 연출: 완전히 시점이 바뀐 후 위젯이 뜨도록
    (Utilities|FlowControl|Delay 1.2)
    ;[1 1 1 1 12] is Valid 체크 해제 시 오버랩되지 않은 플레이어들의 화면에 위젯이 띄워지지 않아 None 오류 출력됨
    (bind _returnvalue_2 (UserInterface|CreateWidget "/Game/Shop/ShopusingBP/WG_Shop.WG_Shop_C" 0 self))
    (Utilities|IsValid _returnvalue_2
      (:Is%20Valid
        (UserInterface|Viewport|AddtoViewport _returnvalue_2 0)
        ;[1 1 1] Flush Input: 체크 해제 시 마지막에 눌린 입력키 효과가 지속됨
        (Input|SetInputModeUIOnly _returnvalue _returnvalue_2 "DoNotLock" true)
        (Variables|/Script/Engine.PlayerController|SetbShowMouseCursor _returnvalue true)))))

(event OnComponentEndOverlap(ShopTriggerBox)
  (params (OverlappedComponent :type Primitive%20Component%20Object%20Reference) (OtherActor :type Actor%20Object%20Reference) (OtherComp :type Primitive%20Component%20Object%20Reference) (OtherBodyIndex :type Integer))
  (bind _asbp_third_person_character (Utilities|Casting|CastToBP_ThirdPersonCharacter OtherActor))
  (Utilities|IsValid _asbp_third_person_character
    (:Is%20Valid
      (Development|PrintString "Bye"))))

(fn ConstructionScript)